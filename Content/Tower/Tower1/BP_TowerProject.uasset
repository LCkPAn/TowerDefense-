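; Tower defense turret that fires BP_Projectile actors at enemies entering its range sphere.
; Sphere overlaps maintain a list of BP_Ennemi; the first entry becomes the target, and Tick yaws the turret mesh toward it.
; A looping timer behind a DoOnce spawns projectiles at the arrow until the list empties.
; Evolution is a print stub, and closest-enemy selection is left unwired.
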(event OnComponentEndOverlap(Sphere)
  (params (OverlappedComponent :type Primitive%20Component%20Object%20Reference) (OtherActor :type Actor%20Object%20Reference) (OtherComp :type Primitive%20Component%20Object%20Reference) (OtherBodyIndex :type Integer))
  (bind _targetmanagement (Variables|Components|GetTargetManagement))
  (Utilities|Casting|CastToBP_Ennemi OtherActor)
  (for (_array_element _array_index) _targetmanagement
    (if (== _array_element OtherActor)
      (Utilities|Array|RemoveIndex (Variables|Components|GetTargetManagement) _array_index)
      (if (== (Utilities|Array|Length _targetmanagement) 0)
        (Variables|Default|SetTargetValide false)
        (CallFunction|StopFire)
        (else
          (CallFunction|FindTarget))))))

(event OnComponentBeginOverlap(Sphere)
  (params (OverlappedComponent :type Primitive%20Component%20Object%20Reference) (OtherActor :type Actor%20Object%20Reference) (OtherComp :type Primitive%20Component%20Object%20Reference) (OtherBodyIndex :type Integer) (bFromSweep :type Boolean) (SweepResult :type Hit%20Result%20Structure%20%28by%20ref%29))
  (bind _asbp_ennemi (Utilities|Casting|CastToBP_Ennemi OtherActor))
  (Variables|Default|SetTargetValide true)
  (Utilities|Array|Add (Variables|Components|GetTargetManagement) _asbp_ennemi)
  (CallFunction|FindTarget)
  (CallFunction|StartFire))

(event Custom|Projectile
  ;[1 1 1] Je créer un projectile sur ma flèche
  (Game|SpawnActorfromClass "/Game/Tower/Tower1/BP_Projectile.BP_Projectile_C" (Transformation|GetWorldTransform (Variables|Default|GetArrow)) "Undefined" 0 0))

(event Custom|StartFire
  ;[1 1 1] Je tire des projectiles
  (Utilities|FlowControl|DoOnce false
    (:Completed
      (CallFunction|Projectile)
      (Utilities|Time|SetTimerbyFunctionName 0 "Projectile" (/ 1.0 (Variables|Components|GetProjectilePerSecond)) true))))

(event Custom|StopFire
  ;[1 1 1] Je tire des projectiles
  (Utilities|Time|ClearTimerbyFunctionName 0 "Projectile")
  (Utilities|FlowControl|DoOnce false) ; enters at Reset
)

(event EventTick
  (params (DeltaSeconds :type Float%20%28single-precision%29))
  (if (Variables|Default|GetTargetValide)
    (CallFunction|TurretRotation DeltaSeconds)))

(event EventEvolution
  (Development|PrintString "Salut"))

(fn ConstructionScript)

(fn TurretRotation
  (params (DeltaSecond :type Float%20%28double-precision%29))
  (Transformation|SetWorldRotation (Variables|Default|GetTowerPower) (Math|Rotator|MakeRotator 0.0 0.0 (+ (.yaw (Math|Interpolation|RInterpTo (Transformation|GetActorRotation) (Math|Rotator|FindLookatRotation (Transformation|GetWorldLocation (Variables|Default|GetTowerPower)) (Transformation|GetActorLocation (Variables|Default|GetTarget))) (Utilities|Time|GetWorldDeltaSeconds) 0.0)) -9e+01)) false false))

(fn FindTarget
  (Variables|Default|SetTarget (Utilities|Array|Get(acopy) (Variables|Components|GetTargetManagement))))