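; BP_TowerBoomer is a tower that fires BP_BoomerArmor projectiles once an enemy (BP_Ennemi) enters its detection sphere.
; StartFire, guarded by a DoOnce, spawns a shot at the Arrow's transform, then repeats it on a looping timer using ProjectilePerSecond as the interval.
; StopFire clears the timer and resets the DoOnce, but nothing in this graph calls it.
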(event OnComponentBeginOverlap(Sphere)
  (params (OverlappedComponent :type Primitive%20Component%20Object%20Reference) (OtherActor :type Actor%20Object%20Reference) (OtherComp :type Primitive%20Component%20Object%20Reference) (OtherBodyIndex :type Integer) (bFromSweep :type Boolean) (SweepResult :type Hit%20Result%20Structure%20%28by%20ref%29))
  (Utilities|Casting|CastToBP_Ennemi OtherActor)
  (CallFunction|StartFire))

(event Custom|Projectile
  ;[1 1 1] Je créer un projectile sur ma flèche
  (Game|SpawnActorfromClass "/Game/Tower/Tower3/BP_BoomerArmor.BP_BoomerArmor_C" (Transformation|GetWorldTransform (Variables|Default|GetArrow)) "Undefined" 0 0))

(event Custom|StartFire
  ;[1 1 1] Je tire des projectiles
  (Utilities|FlowControl|DoOnce false
    (:Completed
      (CallFunction|Projectile)
      (Utilities|Time|SetTimerbyFunctionName 0 "Projectile" (Variables|Default|GetProjectilePerSecond) true))))

(event Custom|StopFire
  ;[1 1 1] Je tire des projectiles
  (Utilities|Time|ClearTimerbyFunctionName 0 "Projectile")
  (Utilities|FlowControl|DoOnce false) ; enters at Reset
)

(fn ConstructionScript)