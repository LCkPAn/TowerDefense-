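; BP_Ennemi is an enemy that travels along the level's BP_Spline and is destroyed when its health runs out.
; On BeginPlay, a Timeline scaled by Time moves it along the spline, with rotation always sampled at the spline's start.
; AffectHealth adds a signed delta through UpdateHealthPoints, prints the result and destroys the actor if DeadEvent flags it dead.
; BeginPlay also passes HealthPoints into that function, doubling starting health.
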(event Custom|DeadEvent
  ;[1 1 1] Verifie ennemi dead
  (if (<= (Variables|Default|GetHealthPoints) 0.0)
    (Variables|Default|SetIsDead true)
    (else
      (Variables|Default|SetIsDead false))))

(event Custom|Move
  (bind _spline (Variables|Default|GetSpline))
  (bind _spline_2 (Variables|/Game/Characters/Spline/BP_Spline.BP_Spline_C|GetSpline _spline))
  ;[1 1 1] MoveSpline
  (Components|Timeline|SetPlayRate (Variables|Default|GetTimeline) (/ 1.0 (Variables|Default|GetTime)))
  (bind _move (Timeline|Timeline Play)
    (:Update
      (Transformation|SetActorTransform (Math|Transform|MakeTransform (Spline|GetLocationatDistanceAlongSpline _spline_2 (Math|Float|Lerp 0.0 (Spline|GetSplineLength (Variables|/Game/Characters/Spline/BP_Spline.BP_Spline_C|GetSpline (Variables|Default|GetSpline))) _move) "World") (Spline|GetRotationatDistanceAlongSpline _spline_2 0.0 "Local") "1.000000,1.000000,1.000000")))))

(event EventAffectHealth
  (params (Dammage :type Float%20%28double-precision%29))
  ;[1 1 1] Gestion dégâts
  (bind _newhealth (CallFunction|UpdateHealthPoints Dammage))
  (Development|PrintString (Utilities|String|ToString(Float) _newhealth))
  (if (Variables|Default|GetIsDead)
    (Actor|DestroyActor)))

(event EventBeginPlay
  ;[1 1 1] MoveSpline
  (bind _returnvalue (Actor|GetActorOfClass "/Game/Characters/Spline/BP_Spline.BP_Spline_C"))
  (Variables|Default|SetSpline _returnvalue)
  (CallFunction|Move)
  (CallFunction|UpdateHealthPoints (Variables|Default|GetHealthPoints)))

(fn ConstructionScript)

(fn UpdateHealthPoints
  (params (Delta :type Float%20%28double-precision%29))
  ;[1 1 1] Set up Heatlh
  (bind _output_get (Variables|Default|SetHealthPoints (+ Delta (Variables|Default|GetHealthPoints))))
  (CallFunction|DeadEvent)
  (return _output_get))