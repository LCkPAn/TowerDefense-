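; BP_FollowSpline is an actor that moves itself along a spline in the level once play begins.
; On BeginPlay it finds a BP_Spline actor by class, then plays a timeline with its rate scaled by the inverse of Time.
; Each update maps the timeline's Move alpha to distance along the spline for world location, while rotation always samples the spline's start in local space.
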(event Custom|Move
  (bind _spline (Variables|Default|GetSpline))
  (bind _spline_2 (Variables|/Game/Characters/Spline/BP_Spline.BP_Spline_C|GetSpline _spline))
  (Components|Timeline|SetPlayRate (Variables|Default|GetTimeline) (/ 1.0 (Variables|Default|GetTime)))
  (bind _move (Timeline|Timeline Play)
    (:Update
      (Transformation|SetActorTransform (Math|Transform|MakeTransform (Spline|GetLocationatDistanceAlongSpline _spline_2 (Math|Float|Lerp 0.0 (Spline|GetSplineLength (Variables|/Game/Characters/Spline/BP_Spline.BP_Spline_C|GetSpline (Variables|Default|GetSpline))) _move) "World") (Spline|GetRotationatDistanceAlongSpline _spline_2 0.0 "Local") "1.000000,1.000000,1.000000")))))

(event EventBeginPlay
  (bind _returnvalue (Actor|GetActorOfClass "/Game/Characters/Spline/BP_Spline.BP_Spline_C"))
  (Variables|Default|SetSpline _returnvalue)
  (CallFunction|Move))

(fn ConstructionScript)